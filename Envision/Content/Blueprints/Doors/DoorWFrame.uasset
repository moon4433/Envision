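; Framed door Blueprint that swings open when a FirstPersonCharacter is inside its trigger box and closes when none remains.
; Tick polls the box's overlaps to play or reverse the OpenAndClose timeline, which sets the door's absolute world yaw.
; Separate begin and end overlap events, unfiltered by actor class, play open and close sounds at the world origin after short delays.
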(event `self.ReceiveTick`
  (params (DeltaSeconds :type "Float (single-precision)"))
  ;[1 1 1] Tell when the door to open
  (if (not (== (`KismetArrayLibrary.Array_Length` (`PrimitiveComponent.GetOverlappingActors` (`self.Box`) "/Game/Blueprints/StartingContent/FirstPersonCharacter.FirstPersonCharacter_C")) 0))
    (bind (_direction _newtrack_0) (`Timeline|openAndClose` :!label _label)
      (:`Update`
        (`SceneComponent.K2_SetWorldRotation` (`self.Door`) (`KismetMathLibrary.MakeRotator` 0.0 0.0 _newtrack_0) false false)))
    (else
      (goto _label :!via `Reverse`))))

(event `self.Box.OnComponentBeginOverlap`
  (params (OverlappedComponent :type "PrimitiveComponent Object Reference") (OtherActor :type "Actor Object Reference") (OtherComp :type "PrimitiveComponent Object Reference") (OtherBodyIndex :type Integer) (bFromSweep :type Boolean) (SweepResult :type "HitResult Structure (by ref)"))
  ;[1 1 1] Tell when to play open sound
  (`KismetSystemLibrary.Delay` 0.05)
  (`GameplayStatics.PlaySoundAtLocation` "/Game/Sounds/DoorsSounds01.DoorsSounds01" (0.0 0.0 0.0) (struct) 1.0 1.0 0.0 null null null))

(event `self.Box.OnComponentEndOverlap`
  (params (OverlappedComponent :type "PrimitiveComponent Object Reference") (OtherActor :type "Actor Object Reference") (OtherComp :type "PrimitiveComponent Object Reference") (OtherBodyIndex :type Integer))
  ;[1 1 1] Tell when to play closing sound
  (`KismetSystemLibrary.Delay` 0.78)
  (`GameplayStatics.PlaySoundAtLocation` "/Game/Sounds/DoorsSounds02.DoorsSounds02" (0.0 0.0 0.0) (struct) 1.0 1.0 0.0 null null null))

(fn `UserConstructionScript`)